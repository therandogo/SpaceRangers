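; Attack component that spawns an attack aimed at player pawn 0, configured by the AttackPDA data asset.
; AttackStartup spawns each FX class at an offset from the owner, then immediately calls AttackExecute.
; AttackExecute spawns the attack Blueprint, passes its tuning values and target through SetParamsMessage, then sets its rotation using a relative look-at toward the player.
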(fn AttackStartup
  (bind _returnvalue (Components|GetOwner))
  (bind _returnvalue_2 (Transformation|GetActorTransform _returnvalue))
  (for _array_element (Variables|/Game/Framework/DataAssests/DA_GenerticAttack.DA_GenerticAttack_C|GetSpawnFX (Variables|AttackParams|GetAttackPDA))
    (Game|SpawnActorfromClass _array_element (Math|Transform|MakeTransform (+ (.location _returnvalue_2) (Variables|AttackParams|GetSpawnFxLocOffset)) (.rotation _returnvalue_2) (.scale _returnvalue_2)) "Undefined" "MultiplyWithRoot" 0 0))
  (CallFunction|AttackExecute))

(fn AttackExecute
  (bind _returnvalue (Components|GetOwner))
  (bind _returnvalue_2 (Game|Player|GetPlayerPawn 0))
  (bind _attackpda (Variables|AttackParams|GetAttackPDA))
  (bind _returnvalue_3 (Transformation|GetActorTransform _returnvalue))
  (bind _returnvalue_4 (Game|SpawnActorfromClass (Variables|/Game/Framework/DataAssests/DA_GenerticAttack.DA_GenerticAttack_C|GetAttackBlueprint (Variables|AttackParams|GetAttackPDA)) (Math|Transform|MakeTransform (+ (.location _returnvalue_3) (Variables|AttackParams|GetAttackSpawnOffset)) (.rotation _returnvalue_3) (.scale _returnvalue_3)) "Undefined" "MultiplyWithRoot" 0 0))
  (bind _output_get (Variables|AttackParams|SetAttackInstance _returnvalue_4))
  (Class|BPIAttackParams|SetParams(Message) _output_get (Variables|/Game/Framework/DataAssests/DA_GenerticAttack.DA_GenerticAttack_C|GetDuration _attackpda) (Variables|/Game/Framework/DataAssests/DA_GenerticAttack.DA_GenerticAttack_C|GetSpeed _attackpda) (Variables|/Game/Framework/DataAssests/DA_GenerticAttack.DA_GenerticAttack_C|GetDmg _attackpda) _returnvalue_2 (Variables|/Game/Framework/DataAssests/DA_GenerticAttack.DA_GenerticAttack_C|GetShootLocation _attackpda))
  (Transformation|SetActorRotation (Variables|AttackParams|GetAttackInstance) (Math|Rotator|FindRelativeLookatRotation (Transformation|GetActorTransform (Variables|AttackParams|GetAttackInstance)) (Transformation|GetActorLocation _returnvalue_2))))