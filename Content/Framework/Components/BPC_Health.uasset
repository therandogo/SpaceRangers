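; Actor component that stores an owner's current and maximum health and exposes functions to damage, heal and query it.
; Initial health uses an override only when it lies between zero and max, otherwise it starts full.
; Healing clamps to max, while damage and the direct setters apply no limits.
; Death is a polled check for health at or below zero, with no events broadcast.
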(fn GetMaxHealth
  (return (Variables|HealthParameters|GetMaxHealth)))

(fn SetMaxHealth
  (params (NewMaxHealth :type Float%20%28double-precision%29))
  (Variables|HealthParameters|SetMaxHealth NewMaxHealth))

(fn SetInitialHealth
  (params (HealthInitialzeOverride :type Float%20%28double-precision%29))
  (if (and (> HealthInitialzeOverride 0.0) (< HealthInitialzeOverride (Variables|HealthParameters|GetMaxHealth)))
    (Variables|HealthParameters|SetCurrentHealth HealthInitialzeOverride)
    (else
      (Variables|HealthParameters|SetCurrentHealth (Variables|HealthParameters|GetMaxHealth)))))

(fn TakeDamage
  (params (DamageRecieved :type Float%20%28double-precision%29))
  (Variables|HealthParameters|SetCurrentHealth (- (Variables|HealthParameters|GetCurrentHealth) DamageRecieved)))

(fn HealDamage
  (params (HealRecieved :type Float%20%28double-precision%29))
  (bind _output_get (Variables|HealthParameters|SetCurrentHealth (+ HealRecieved (Variables|HealthParameters|GetCurrentHealth))))
  (if (> _output_get (Variables|HealthParameters|GetMaxHealth))
    (Variables|HealthParameters|SetCurrentHealth (Variables|HealthParameters|GetMaxHealth))))

(fn GetCurrentHealth
  (return (Variables|HealthParameters|GetCurrentHealth)))

(fn SetCurrentHealth
  (params (CurrentHealthValue :type Float%20%28double-precision%29))
  (Variables|HealthParameters|SetCurrentHealth CurrentHealthValue))

(fn IsDeadCheck
  (if (<= (Variables|HealthParameters|GetCurrentHealth) 0.0)
    (return true)
    (else
      (return false))))