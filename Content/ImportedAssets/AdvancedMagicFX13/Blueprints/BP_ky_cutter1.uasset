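; BP_ky_cutter1 is a magic FX projectile that travels from its FX start point to a location passed through SetParams.
; A timeline lerps the actor over a time set by Speed and destroys it on arrival, alongside a polling loop that deactivates it if Duration is negative.
; Overlapping actors not tagged "ky_shot" spawn color-synced hit emitters; only the MoreEffects branch adds a second emitter and destroys the projectile.
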(event Custom|Move
  ;[1 1 1] New Move Control
  (Utilities|FlowControl|Delay 0.1)
  (Components|Timeline|SetPlayRate (Variables|Default|GetMove%20Timline) (/ 1.0 (Variables|Default|GetSpeed_0)))
  (bind _newtrack_0 (Timeline|Move%20Timline PlayFromStart)
    (:Update
      (Transformation|SetActorLocation (Math|Vector|Lerp(Vector) (Variables|Default|GetStartLocation) (Variables|Default|GetShootLoc) _newtrack_0) false false))
    (:Finished
      (Actor|DestroyActor))))

(event EventBeginPlay
  (Variables|Default|SetStartLocation (Transformation|GetWorldLocation (Variables|Default|GetFX)))
  (CallFunction|Move)
  ;[1 1 1] effect move correct
  (bind _valuecorrect (Timeline|Timeline_0 PlayFromStart)
    (:Update
      (Variables|Default|SetspeedCorrect _valuecorrect)
      ;[1 1 1] duration control
      (Utilities|FlowControl|Delay 0.1 :!label _label)
      (if (< (Variables|Default|Getduration) 0.0)
        ;[1 1 1] fx deactivate
        (Collision|SetCollisionEnabled (Variables|Default|GetBox) "NoCollision")
        (Components|Activation|Deactivate (Variables|Default|GetFX))
        ;[1 1 1] effect destroy
        (Utilities|FlowControl|Delay 1.0)
        (Actor|DestroyActor)
        (else
          (goto _label))))))

(event Collision|EventActorBeginOverlap
  (params (OtherActor :type Actor%20Object%20Reference))
  (bind _hitpoint (Variables|Default|GethitPoint))
  (bind _returnvalue (Transformation|GetWorldLocation _hitpoint))
  ;[1 1 1] spawn collison fx
  (if (Utilities|IsValid OtherActor)
    (if (Utilities|Name|NotEqual(Name) (Utilities|Array|Get(acopy) (Variables|/Script/Engine.Actor|GetTags OtherActor)) "ky_shot")
      (bind _returnvalue_2 (Effects|SpawnEmitteratLocation (Variables|Default|GethitFx) _returnvalue))
      ;[1 1 1] collison fx color sync
      (Effects|Components|ParticleSystem|SetVectorParameter _returnvalue_2 "color" (Math|Conversions|ToVector(LinearColor) (Variables|Default|Getcolor)))
      (if (Variables|Default|GetMore%20Effects)
        (bind _returnvalue_3 (Effects|SpawnEmitteratLocation (Variables|Default|GethitFx1) _returnvalue))
        (Effects|Components|ParticleSystem|SetVectorParameter _returnvalue_3 "color" (Math|Conversions|ToVector(LinearColor) (Variables|Default|Getcolor)))
        (Actor|DestroyActor)))))

(event EventSetParams
  (params (Duration :type Float%20%28double-precision%29) (Speed :type Float%20%28double-precision%29) (Dmg :type Float%20%28double-precision%29) (TargetActor :type Actor%20Object%20Reference) (ShootLocation :type Vector :default "0, 0, 0"))
  (Variables|Default|Setduration Duration)
  (Variables|Default|SetSpeed_0 Speed)
  (Variables|Default|SetShootLoc ShootLocation))

(fn ConstructionScript
  ;[1 1 1] color control
  (Effects|Components|ParticleSystem|SetVectorParameter (Variables|Default|GetFX) "color" (Math|Conversions|ToVector(LinearColor) (Variables|Default|Getcolor))))