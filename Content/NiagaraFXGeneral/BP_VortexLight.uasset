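; BP_VortexLight is a light actor whose mesh color shimmers through random magenta and purple tones.
; The construction script creates a dynamic MI_Light instance, and Tick lerps its Color parameter toward a new random tint by delta time.
; MoveLight bounces TravellingLight back and forth along local X between two limits, but its looping timer is disconnected.
; The direct random SetLightColor call is also disconnected, so only the material color changes.
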(event Custom|MoveLight
  (bind _travelling_light (Variables|Default|GetTravelling%20Light))
  (bind _relativelocation (Variables|/Script/Engine.SceneComponent|GetRelativeLocation _travelling_light))
  (if (> (.x _relativelocation) 3e+04)
    (Variables|Default|SetE_LightMove "NewEnumerator1")
    (elif (< (.x _relativelocation) -3e+04)
      (Variables|Default|SetE_LightMove "NewEnumerator0")))
  (switch Utilities|FlowControl|Switch|SwitchonE_LightMove (Variables|Default|GetE_LightMove)
    (:NewEnumerator0
      (Transformation|AddLocalOffset (Variables|Default|GetTravelling%20Light) (* "1.000000,0.000000,0.000000" 1e+02) false false))
    (:NewEnumerator1
      (Transformation|AddLocalOffset (Variables|Default|GetTravelling%20Light) (* "-1.000000,0.000000,0.000000" 1e+02) false false))))

(event EventTick
  (params (DeltaSeconds :type Float%20%28single-precision%29))
  (bind _material (Variables|Default|GetMaterial))
  (bind _returnvalue (Rendering|Material|GetVectorParameterValue _material "Color" :!class /Script/Engine.MaterialInstanceDynamic))
  (Rendering|Material|SetVectorParameterValue _material "Color" (Math|Color|Lerp(LinearColor) _returnvalue (Utilities|Struct|MakeLinearColor (Math|Random|RandomFloatinRange 0.5 1.0) (Math|Random|RandomFloatinRange 0.0 0.2) (Math|Random|RandomFloatinRange 0.5 1.0) 1.0) DeltaSeconds) :!class /Script/Engine.MaterialInstanceDynamic))

(event EventBeginPlay)

(fn ConstructionScript
  (bind _returnvalue (Rendering|Material|CreateDynamicMaterialInstance (Variables|Default|GetStaticMesh) 0 "/Game/Skybox/Mats/MI_Light.MI_Light" "None" :!class /Script/Engine.PrimitiveComponent))
  (Variables|Default|SetMaterial _returnvalue))